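; Stage 1 zombie character Blueprint that handles visual hit feedback: damage numbers, gore and blood splatter.
; OnScreenDamage spawns a DamageWidget at the capsule's projected screen position.
; OnBloodEffectEvent hides the Head bone and attaches a blood emitter there on headshots, otherwise attaching a blood emitter to the mesh.
; That emitter's particle collisions spawn temporary, randomly sized decals aligned to the surface normal, using dynamic materials with a random frame.
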(event Custom|Collider
  (params (EventName :type Name) (EmitterTime :type Float%20%28single-precision%29) (ParticleTime :type Integer) (Location :type Vector) (Velocity :type Vector) (Direction :type Vector) (Normal :type Vector) (BoneName :type Name) (PhysMat :type Physical%20Material%20Object%20Reference))
  (bind _returnvalue (Rendering|Material|CreateDynamicMaterialInstance "/Game/Bluprints/Effect/BloodDecal_Material.BloodDecal_Material" :!class /Script/Engine.KismetMaterialLibrary))
  (Rendering|Material|SetScalarParameterValue _returnvalue "Frame" (Math|Conversions|ToFloat(Integer) (Math|Random|RandomInteger 11)) :!class /Script/Engine.MaterialInstanceDynamic)
  (Rendering|Decal|SpawnDecalatLocation _returnvalue (Math|Conversions|ToVector(Float) (Math|Random|RandomFloatinRange 5e+01 2e+02)) Location (Math|Conversions|RotationFromXVector Normal) 2e+01))

(event EventBeginPlay)

(event Collision|EventActorBeginOverlap
  (params (OtherActor :type Actor%20Object%20Reference)))

(event EventOnBloodEffectEvent
  (params (HitResult :type Hit%20Result%20Structure))
  (bind _hitbonename (Collision|BreakHitResult HitResult))
  (bind _mesh (Variables|Character|GetMesh))
  (if (Utilities|Name|Equal(Name) _hitbonename "Head")
    (Components|SkinnedMesh|HideBonebyName _mesh "Head" "PBO_None")
    (Effects|SpawnEmitterAttached "/Game/Bluprints/Effect/P_body_bullet_NoStop.P_body_bullet_NoStop" _mesh _hitbonename "0, 0, 0" "90.000000,0.000000, 0")
    (else
      (bind _returnvalue (Effects|SpawnEmitterAttached "/Game/Bluprints/Effect/BloodEfect.BloodEfect" (Variables|Character|GetMesh) "None"))
      (EventDispatchers|BindEventtoOnParticleCollide _returnvalue (delegate Custom|Collider)))))

(event EventTick
  (params (DeltaSeconds :type Float%20%28single-precision%29)))

(event EventOnScreenDamage
  (params (FlictDamage :type Float%20%28single-precision%29))
  (CallFunction|SpawnFloatingCombatText (Transformation|GetWorldLocation (Variables|Default|GetCapsuleComponent)) FlictDamage))

(fn ConstructionScript)

(fn SpawnFloatingCombatText
  (params (WorldLocation :type Vector) (Damage :type Float%20%28single-precision%29))
  (bind _returnvalue (UserInterface|CreateWidget "/Game/UI/HUD/DamageWidget.DamageWidget_C" 0 (.ScreenPosition (Class|GameplayStatics|ProjectWorldtoScreen (Game|GetPlayerController 0) WorldLocation false)) Damage))
  (UserInterface|Viewport|AddtoViewport _returnvalue 0))
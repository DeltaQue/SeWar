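; Controller Blueprint, RyzenController_BP, that handles the player's inventory screen.
; The OpenInventory input creates and shows a WB_Inventory widget when the stored reference is invalid, and removes it from its parent when valid.
; The branch tests validity, not visibility, and never clears the reference on removal.
; ReloadInventory tells an existing widget to reload its items through LoadInventoryItem.
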(event EventReloadInventory
  (bind _inventory_widget (Variables|Default|GetInventory%20WIdget))
  (Utilities|IsValid _inventory_widget
    (:Is%20Valid
      (bind _aswb_inventory (Utilities|Casting|CastToWB_Inventory _inventory_widget))
      (Default|LoadInventoryItem _aswb_inventory))))

(event Input|ActionEvents|InputActionOpenInventory
  (params (Key :type Key%20Structure))
  ;[1 1 1] 인벤토리 오픈 I 를 눌렀을때
  (:Pressed
    (if (Utilities|IsValid (Variables|Default|GetInventory%20WIdget))
      (Widget|RemovefromParent (Variables|Default|GetInventory%20WIdget))
      (else
        (Utilities|IsValid (Variables|Default|GetInventory%20WIdget)
          (:Is%20Valid
            _)
          (:Is%20Not%20Valid
            (bind _returnvalue (UserInterface|CreateWidget "/Game/UserInterface/WB_Inventory.WB_Inventory_C"))
            (Variables|Default|SetInventory%20WIdget _returnvalue)))
        (UserInterface|Viewport|AddtoViewport (Variables|Default|GetInventory%20WIdget) 0)))))

(fn ConstructionScript)